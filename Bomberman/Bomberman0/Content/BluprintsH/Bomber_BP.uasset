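; Player-side Bomberman-style Blueprint that drops bombs and handles the player's death.
; F calls Spawn to place a bomb, while Q and H print the coin count and health as debug readouts.
; Health is read from the Healt component and also printed on any damage.
; Tick polls that health and, at zero or below, pauses the game and shows the Death widget with UI-only input and mouse cursor.
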(event `Key|Q`
  (params (Key :type "Key Structure"))
  ;[1 1 1] Saber monedas
  (:`Pressed`
    (`KismetSystemLibrary.PrintString` (`KismetStringLibrary.Conv_IntToString` (`self.Monedas`)))))

(event `self.ReceiveTick`
  (params (DeltaSeconds :type "Float (single-precision)"))
  (bind _returnvalue (`GameplayStatics.GetPlayerController` 0))
  ;[1 1 1] Evento de muerte y pantalla de muerte
  (if (<= (`Healt.Sald` (`self.Healt`)) 0.0)
    (`GameplayStatics.SetGamePaused` true)
    (bind _returnvalue_2 (`|CreateWidget` "/Game/UI/Death.Death_C" (`GameplayStatics.GetPlayerController` 0)))
    (`UserWidget.AddToPlayerScreen` _returnvalue_2 0)
    (`WidgetBlueprintLibrary.SetInputMode_UIOnlyEx` _returnvalue _returnvalue_2)
    (set `PlayerController.bShowMouseCursor` true _returnvalue)))

(event `Key|F`
  (params (Key :type "Key Structure"))
  ;[1 1 1] Spawnear bomba
  (:`Pressed`
    (`self.Spawn`)))

(event `self.ReceiveAnyDamage`
  (params (Damage :type "Float (single-precision)") (DamageType :type "DamageType Object Reference") (InstigatedBy :type "Controller Object Reference") (DamageCauser :type "Actor Object Reference"))
  ;[1 1 1] Para que imprima la salud cada vez que se hace daño
  (`KismetSystemLibrary.PrintString` (`KismetStringLibrary.Conv_DoubleToString` (`Healt.Sald` (`self.Healt`)))))

(event `Key|H`
  (params (Key :type "Key Structure"))
  ;[1 1 1] Saber salud
  (:`Pressed`
    (`KismetSystemLibrary.PrintString` (`KismetStringLibrary.Conv_DoubleToString` (`Healt.Sald` (`self.Healt`))))))

(fn `UserConstructionScript`)